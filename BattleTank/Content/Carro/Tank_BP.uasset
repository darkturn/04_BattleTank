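; Player-controllable tank pawn Blueprint that wires movement, aiming, firing and a health bar widget.
; On BeginPlay it initialises TankAiming with barrel and turret, TankMovement with both tracks, and hands itself to the HealthBar widget.
; Move and Turn axes feed movement intents to TankMovement, while Fire triggers TankAiming.
; Aim axes rotate an azimuth gimbal and spring arm, scaled by delta time for frame-rate-independent control.
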(event `self.ReceiveBeginPlay`
  (`TankAimingComponent.Initialise` (`self.TankAiming`) (`self.Barrel`) (`self.Turret`))
  (`TankMovementComponent.Initialise` (`self.TankMovement`) (`self.LeftTrack`) (`self.RightTrack`))
  (`self.InitialiseHealthBarWidget`))

(event `InputAxis|AimAzimuth`
  (params (AxisValue :type "Float (single-precision)"))
  ;[1 1 1] Setup Input di mira
  (`SceneComponent.K2_AddLocalRotation` (`self.Azimuth Gimbal`) (`KismetMathLibrary.MakeRotator` 0.0 0.0 (* AxisValue (`GameplayStatics.GetWorldDeltaSeconds`) 100.0)) false false))

(event `InputAxis|Move`
  (params (AxisValue :type "Float (single-precision)"))
  ;[1 1 1] Setup Input di movimento
  (`TankMovementComponent.IntendMove` (`self.TankMovement`) AxisValue))

(event `InputAxis|Turn`
  (params (AxisValue :type "Float (single-precision)"))
  ;[1 1 1] Setup Input di movimento
  (`TankMovementComponent.IntendTurn` (`self.TankMovement`) AxisValue))

(event `InputAxis|AimElevation`
  (params (AxisValue :type "Float (single-precision)"))
  ;[1 1 1] Setup Input di mira
  (`SceneComponent.K2_AddLocalRotation` (`self.SpringArm`) (`KismetMathLibrary.MakeRotator` 0.0 (* AxisValue (`GameplayStatics.GetWorldDeltaSeconds`) 100.0)) false false))

(event `InputAction|Fire`
  (params (Key :type "Key Structure"))
  ;[1 1 1] Setup Input di mira
  (:`Pressed`
    (`TankAimingComponent.Fire` (`self.TankAiming`))))

(fn `InitialiseHealthBarWidget`
  (bind _ashealth_bar (cast `/Game/UI/HealthBar` (`WidgetComponent.GetUserWidgetObject` (`self.Health Bar`))))
  (set `/Game/UI/HealthBar.MyTank` self _ashealth_bar)
  (return))

(fn `UserConstructionScript`)